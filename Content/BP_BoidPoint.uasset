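; BP_BoidPoint is an actor that acts as a spherical avoidance point for the boids in TargetBoids.
; On BeginPlay and every Tick it packs the Sphere component's world location and scaled radius into a Vector4 and passes it to AddPointAvoidance at its Index, so changes to the sphere carry through at runtime.
; The construction script is empty, with a disconnected copy of the call.
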(event EventBeginPlay
  (bind _sphere (Variables|Default|GetSphere))
  (bind _returnvalue (Transformation|GetWorldLocation _sphere))
  (bind (_x _y _z) (Math|Vector|BreakVector _returnvalue))
  (Default|AddPointAvoidance (Variables|Default|GetTargetBoids) (Math|Vector4|MakeVector4 _x _y _z (Components|Sphere|GetScaledSphereRadius _sphere)) (Variables|Default|GetIndex)))

(event EventTick
  (params (DeltaSeconds :type Float%20%28single-precision%29))
  (bind _sphere (Variables|Default|GetSphere))
  (bind _returnvalue (Transformation|GetWorldLocation _sphere))
  (bind (_x _y _z) (Math|Vector|BreakVector _returnvalue))
  (Default|AddPointAvoidance (Variables|Default|GetTargetBoids) (Math|Vector4|MakeVector4 _x _y _z (Components|Sphere|GetScaledSphereRadius _sphere)) (Variables|Default|GetIndex)))

(fn ConstructionScript)