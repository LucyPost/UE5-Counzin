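; Boids flocking actor that drives the PBoids Niagara system inside a box volume.
; The construction script pushes bounds, count, speed, acceleration and steering parameters into Niagara, scales attraction and orientation radii by MeshScale, and sizes the Box to match.
; Type selects preset flock behaviours (swarm, ring, dynamic or highly parallel) or custom values through getter functions.
; AddPointAvoidance writes a Vector4 avoidance point into one of two Niagara slots by index.
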(event EventBeginPlay)

(fn ConstructionScript
  (bind _p_boids (Variables|Default|GetP_Boids))
  (bind _p_boids_2 (Variables|Default|GetP_Boids))
  (bind _p_boids_3 (Variables|Default|GetP_Boids))
  (bind _p_boids_4 (Variables|Default|GetP_Boids))
  (bind _p_boids_5 (Variables|Default|GetP_Boids))
  (bind _p_boids_6 (Variables|Default|GetP_Boids))
  (Niagara|SetNiagaraVariable(Float) _p_boids_3 "WidthX" (Variables|Init|GetWidthX))
  (Niagara|SetNiagaraVariable(Float) _p_boids_3 "WidthY" (Variables|Init|GetWidthY))
  (Niagara|SetNiagaraVariable(Float) _p_boids_3 "Height" (Variables|Init|GetHeight))
  (Niagara|SetNiagaraVariable(Float) _p_boids_4 "AlignmentStrength" (CallFunction|GetAlignmentStrength))
  (Niagara|SetNiagaraVariable(Float) _p_boids_4 "AttractionStrength" (CallFunction|GetAttractionStrength))
  (Niagara|SetNiagaraVariable(Float) _p_boids_4 "RepulsionStrength" (Variables|Boids|GetRepulsionStrength))
  (Niagara|SetNiagaraVariable(Float) _p_boids_6 "ZoaRadius" (* (CallFunction|GetZoaRadius) (Variables|init|GetMeshScale)))
  (Niagara|SetNiagaraVariable(Float) _p_boids_6 "ZooRadius" (* (CallFunction|GetZooRadius) (Variables|init|GetMeshScale)))
  (Niagara|SetNiagaraVariable(Float) _p_boids_6 "ZorRadiusOuter" (Variables|Boids|GetZorRadiusOuter))
  (Niagara|SetNiagaraVariable(Float) _p_boids_6 "ZorRadiusInner" (Variables|Boids|GetZorRadiusInner))
  (Class|NiagaraComponent|SetVariableInt _p_boids "BoidsNum" (Variables|init|GetBoidsNum))
  (Niagara|SetNiagaraVariable(Float) _p_boids "BaseIniSpeed" (Variables|init|GetBaseIniSpeed))
  (Niagara|SetNiagaraVariable(Vector3) _p_boids "MinIniVelocity" (Variables|init|GetMinIniVelocity))
  (Niagara|SetNiagaraVariable(Vector3) _p_boids "MaxIniVelocity" (Variables|init|GetMaxIniVelocity))
  (Niagara|SetNiagaraVariable(Vector3) _p_boids_2 "MinAcceleration" (Variables|Movemont|GetMinAcceleration))
  (Niagara|SetNiagaraVariable(Vector3) _p_boids_2 "MaxAcceleration" (Variables|Movemont|GetMaxAcceleration))
  (Niagara|SetNiagaraVariable(Float) _p_boids_2 "IntrestedSpeed" (Variables|Movemont|GetIntrestedSpeed))
  (Niagara|SetNiagaraVariable(Float) _p_boids_2 "MaxSpeed" (Variables|Movemont|GetMaxSpeed))
  (Niagara|SetNiagaraVariable(Float) _p_boids_5 "HalfAngleOfSight" (CallFunction|GetHalfAngleOfSight))
  (Niagara|SetNiagaraVariable(Float) _p_boids_5 "MeshScale" (Variables|init|GetMeshScale))
  (Components|Box|SetBoxExtent (Variables|Default|GetBox) (* (Math|Vector|MakeVector (Variables|Init|GetWidthX) (Variables|Init|GetWidthY) (Variables|Init|GetHeight)) 0.5) true))

(fn AddPointAvoidance
  (params (PointData :type Vector%204%20Structure) (Index :type Integer))
  (bind _p_boids (Variables|Default|GetP_Boids))
  (switch int Index
    (:0
      (Class|NiagaraComponent|SetVariableVec4 _p_boids "PointAvoidanceData01" PointData))
    (:1
      (Class|NiagaraComponent|SetVariableVec4 _p_boids "PointAvoidanceData02" PointData))))

(fn GetAttractionStrength
  (switch Utilities|FlowControl|Switch|SwitchonE_BoidsType (Variables|Presets|GetType)
    (:NewEnumerator0
      (return (Variables|Boids|GetAttractionStrength)))
    (:NewEnumerator1
      (return 1.0))
    (:NewEnumerator2
      (return 0.5))
    (:NewEnumerator3
      (return 0.5))
    (:NewEnumerator4
      (return 0.5))))

(fn GetAlignmentStrength
  (switch Utilities|FlowControl|Switch|SwitchonE_BoidsType (Variables|Presets|GetType)
    (:NewEnumerator0
      (return (Variables|Boids|GetAlignmentStrength)))
    (:NewEnumerator1
      (return 0.5))
    (:NewEnumerator2
      (return 1.0))
    (:NewEnumerator3
      (return 1.0))
    (:NewEnumerator4
      (return 1.0))))

(fn GetZoaRadius
  (switch Utilities|FlowControl|Switch|SwitchonE_BoidsType (Variables|Presets|GetType)
    (:NewEnumerator0
      (return (Variables|Boids|GetZoaRadius)))
    (:NewEnumerator1
      (return 3.6e+02))
    (:NewEnumerator2
      (return 8e+02))
    (:NewEnumerator3
      (return 7e+02))
    (:NewEnumerator4
      (return 5.5e+02))))

(fn GetZooRadius
  (switch Utilities|FlowControl|Switch|SwitchonE_BoidsType (Variables|Presets|GetType)
    (:NewEnumerator0
      (return (Variables|Boids|GetZooRadius)))
    (:NewEnumerator1
      (return 175.0))
    (:NewEnumerator2
      (return 1.8e+02))
    (:NewEnumerator3
      (return 3e+02))
    (:NewEnumerator4
      (return 3.6e+02))))

(fn GetHalfAngleOfSight
  (switch Utilities|FlowControl|Switch|SwitchonE_BoidsType (Variables|Presets|GetType)
    (:NewEnumerator0
      (return (Variables|Boids|GetHalfAngleOfSight)))
    (:NewEnumerator1
      (return 95.0))
    (:NewEnumerator2
      (return 1.5e+02))
    (:NewEnumerator3
      (return 95.0))
    (:NewEnumerator4
      (return 95.0))))