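; BP_MovingCone is an actor that wanders smoothly around its spawn point, pointing along its direction of travel.
; BeginPlay stores the start location, then Tick samples three decorrelated 1D Perlin noise channels over game time, shifted by an Offset variable, to set its position.
; Each frame it rotates using a look-at from the previous location to the new one.
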(event EventBeginPlay
  (bind _output_get (Variables|Default|SetStartLoc (Transformation|GetActorLocation)))
  (bind _output_get_2 (Variables|Default|SetPreLoc _output_get))
  (Variables|Default|SetCurrentLoc _output_get_2))

(event EventTick
  (params (DeltaSeconds :type Float%20%28single-precision%29))
  (bind _returnvalue (Utilities|Time|GetGameTimeinSeconds))
  (bind _offset (Variables|Default|GetOffset))
  (bind _returnvalue_2 (* _returnvalue 0.2))
  (bind _output_get (Variables|Default|SetCurrentLoc (+ (Variables|Default|GetStartLoc) (* (Math|Vector|MakeVector (Class|KismetMathLibrary|PerlinNoise1D (+ _returnvalue_2 _offset)) (Class|KismetMathLibrary|PerlinNoise1D (* (+ _returnvalue_2 2e+02 _offset) 1.05)) (Class|KismetMathLibrary|PerlinNoise1D (* (+ _returnvalue_2 4e+03 _offset) 0.95))) 1.5e+03))))
  (Transformation|SetActorLocation _output_get false false)
  (Transformation|SetActorRotation (Math|Rotator|FindLookatRotation (Variables|Default|GetPreLoc) (Variables|Default|GetCurrentLoc)))
  (Variables|Default|SetPreLoc (Variables|Default|GetCurrentLoc)))

(fn ConstructionScript)